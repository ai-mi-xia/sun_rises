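; BP_Puddles9 is a water puddle pickup that gives each player its water once when their character overlaps its sphere.
; The overlap first tells that player's main controller to change the water light via a client call.
; On authority, an OverlappedPuddle9 flag in the player state gates adding water to the controller, updating the HUD, raising character opacity and playing a collect sound.
; An older player-state-based version is left disconnected.
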(event `self.SphereCollision.OnComponentBeginOverlap`
  (params (OverlappedComponent :type "PrimitiveComponent Object Reference") (OtherActor :type "Actor Object Reference") (OtherComp :type "PrimitiveComponent Object Reference") (OtherBodyIndex :type Integer) (bFromSweep :type Boolean) (SweepResult :type "HitResult Structure (by ref)"))
  (bind _puddlewateramt (`self.PuddleWaterAmt`))
  ;[1 1 1] Player 1 Collision
  (bind _asbp_third_person_character (cast `/Game/Blueprints/Character/BP_ThirdPerson_Character` OtherActor)) ; Get the Player State of the overlapping Character
  (bind _asbp_default_player_state (cast `/Game/Blueprints/Framework/BP_Default_PlayerState` (`Pawn.PlayerState` _asbp_third_person_character))) ; Set variables for that Player
  (bind _asbp_pc_main_controller (cast `/Game/Blueprints/Framework/BP_PC_MainController` (`self.GetInstigatorController` OtherActor)))
  (`/Game/Blueprints/Framework/BP_PC_MainController.Client_ChangeWaterLight` _asbp_pc_main_controller (`ActorComponent.GetOwner` OverlappedComponent))
  (`/Engine/EditorBlueprintResources/ActorMacros.Switch Has Authority` ; moved this so I can call the RPC First
    (:`Authority`
      (if (not (`/Game/Blueprints/Framework/BP_Default_PlayerState.OverlappedPuddle9?` _asbp_default_player_state))
        (set `/Game/Blueprints/Framework/BP_PC_MainController.Water` (+ (`/Game/Blueprints/Framework/BP_PC_MainController.Water` _asbp_pc_main_controller) _puddlewateramt) _asbp_pc_main_controller)
        (set `/Game/Blueprints/Framework/BP_Default_PlayerState.OverlappedPuddle9?` true _asbp_default_player_state)
        (`/Game/Blueprints/Framework/BP_PC_MainController.Multicast_CallHUD` _asbp_pc_main_controller)
        (`/Game/Blueprints/Framework/BP_PC_MainController.IncreaseCharaOpacity` _asbp_pc_main_controller (`KismetMathLibrary.Conv_IntToDouble` _puddlewateramt))
        (`/Game/Blueprints/Framework/BP_PC_MainController.Client_PlayWaterCollectSound` _asbp_pc_main_controller)))))

(fn `UserConstructionScript`)