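; BP_PuddlesTest is a test puddle interactable with separate collision spheres for Player 1 and Player 2, apparently meant to add water to player controllers.
; On server-side overlap, each sphere checks the instigating controller's position in the game mode's controller list against that player's index array.
; A match currently does nothing: the water addition and sphere destruction nodes are disconnected.
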(event `self.SphereCollisionP1.OnComponentBeginOverlap`
  (params (OverlappedComponent :type "PrimitiveComponent Object Reference") (OtherActor :type "Actor Object Reference") (OtherComp :type "PrimitiveComponent Object Reference") (OtherBodyIndex :type Integer) (bFromSweep :type Boolean) (SweepResult :type "HitResult Structure (by ref)"))
  ;[1 1 1] Player 1 Collision
  (`/Engine/EditorBlueprintResources/ActorMacros.Switch Has Authority`
    (:`Authority`
      (bind _asbp_pc_main_controller (cast `/Game/Blueprints/Framework/BP_PC_MainController` (`self.GetInstigatorController` OtherActor))) ; change water amount on player controller
      (bind _asbp_gm_default (cast `/Game/Blueprints/Framework/BP_GM_Default` (`GameplayStatics.GetGameMode`)))
      (for _array_element (`/Game/Blueprints/Framework/BP_GM_Default.Player1Indexes` _asbp_gm_default)
        (if (== (`KismetArrayLibrary.Array_Find` (`/Game/Blueprints/Framework/BP_GM_Default.AllPlayerControllers` _asbp_gm_default) _asbp_pc_main_controller) _array_element)
          _)))))

(event `self.SphereCollisionP2.OnComponentBeginOverlap`
  (params (OverlappedComponent :type "PrimitiveComponent Object Reference") (OtherActor :type "Actor Object Reference") (OtherComp :type "PrimitiveComponent Object Reference") (OtherBodyIndex :type Integer) (bFromSweep :type Boolean) (SweepResult :type "HitResult Structure (by ref)"))
  ;[1 1 1] Player 2 Collision
  (`/Engine/EditorBlueprintResources/ActorMacros.Switch Has Authority`
    (:`Authority`
      (bind _asbp_pc_main_controller (cast `/Game/Blueprints/Framework/BP_PC_MainController` (`self.GetInstigatorController` OtherActor))) ; change water amount on player controller
      (bind _asbp_gm_default (cast `/Game/Blueprints/Framework/BP_GM_Default` (`GameplayStatics.GetGameMode`)))
      (for _array_element (`/Game/Blueprints/Framework/BP_GM_Default.Player2Indexes` _asbp_gm_default)
        (if (== (`KismetArrayLibrary.Array_Find` (`/Game/Blueprints/Framework/BP_GM_Default.AllPlayerControllers` _asbp_gm_default) _asbp_pc_main_controller) _array_element)
          _)))))

(fn `UserConstructionScript`)