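; BP_BloomTreeCollision is an interactable trigger volume marking a bloom spot for third-person player characters.
; On overlap, if the player's controller has enough flowers, it stores the overlapping actor on controller and character and calls ServerPressHeartUI.
; Leaving clears both references and calls ServerStopHeartPulse, regardless of flower count.
; The stored reference is the overlapping character itself, and the player state cast only gates execution.
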(event `self.BloomCollision.OnComponentBeginOverlap`
  (params (OverlappedComponent :type "PrimitiveComponent Object Reference") (OtherActor :type "Actor Object Reference") (OtherComp :type "PrimitiveComponent Object Reference") (OtherBodyIndex :type Integer) (bFromSweep :type Boolean) (SweepResult :type "HitResult Structure (by ref)"))
  ;[1 1 1] Begin Overlap
  (bind _asbp_third_person_character (cast `/Game/Blueprints/Character/BP_ThirdPerson_Character` OtherActor)) ; Get the Player State of the overlapping Character
  (cast `/Game/Blueprints/Framework/BP_Default_PlayerState` (`Pawn.PlayerState` _asbp_third_person_character)) ; Set variables for that Player
  (bind _asbp_pc_main_controller (cast `/Game/Blueprints/Framework/BP_PC_MainController` (`self.GetInstigatorController` OtherActor)))
  (if (>= (`/Game/Blueprints/Framework/BP_PC_MainController.FlowerCount` _asbp_pc_main_controller) 6)
    (set `/Game/Blueprints/Framework/BP_PC_MainController.BloomSpot_OverlappedActor` OtherActor _asbp_pc_main_controller)
    (set `/Game/Blueprints/Character/BP_ThirdPerson_Character.BloomSpotCBP` OtherActor _asbp_third_person_character)
    (`/Game/Blueprints/Framework/BP_PC_MainController.Server_PressHeartUI` _asbp_pc_main_controller)))

(event `self.BloomCollision.OnComponentEndOverlap`
  (params (OverlappedComponent :type "PrimitiveComponent Object Reference") (OtherActor :type "Actor Object Reference") (OtherComp :type "PrimitiveComponent Object Reference") (OtherBodyIndex :type Integer))
  ;[1 1 1] End Overlap
  (bind _asbp_third_person_character (cast `/Game/Blueprints/Character/BP_ThirdPerson_Character` OtherActor)) ; Get the Player State of the overlapping Character
  (cast `/Game/Blueprints/Framework/BP_Default_PlayerState` (`Pawn.PlayerState` _asbp_third_person_character)) ; Set variables for that Player
  (bind _asbp_pc_main_controller (cast `/Game/Blueprints/Framework/BP_PC_MainController` (`self.GetInstigatorController` OtherActor)))
  (set `/Game/Blueprints/Framework/BP_PC_MainController.BloomSpot_OverlappedActor` null _asbp_pc_main_controller)
  (set `/Game/Blueprints/Character/BP_ThirdPerson_Character.BloomSpotCBP` null _asbp_third_person_character)
  (`/Game/Blueprints/Framework/BP_PC_MainController.Server_StopHeartPulse` _asbp_pc_main_controller))

(fn `UserConstructionScript`)