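; BP_DrySpot_Parent is a parent interactable for dry spots that shows and hides flower UI as players enter and leave its collision sphere.
; On the server, entering stores the overlapping actor and component on the BP_PC_MainController and calls ServerAddFlowerUI.
; For a BP_ThirdPerson_Character, leaving clears those references, calls ServerRemoveFlowerUI and hides the character's FlowerSpawn component.
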(event `self.Collision_Sphere.OnComponentBeginOverlap`
  (params (OverlappedComponent :type "PrimitiveComponent Object Reference") (OtherActor :type "Actor Object Reference") (OtherComp :type "PrimitiveComponent Object Reference") (OtherBodyIndex :type Integer) (bFromSweep :type Boolean) (SweepResult :type "HitResult Structure (by ref)"))
  ;[1 1 1] Begin Overlap
  (`/Engine/EditorBlueprintResources/ActorMacros.Switch Has Authority`
    (:`Authority`
      (bind _asbp_pc_main_controller (cast `/Game/Blueprints/Framework/BP_PC_MainController` (`self.GetInstigatorController` OtherActor)))
      (set `/Game/Blueprints/Framework/BP_PC_MainController.DrySpot_OverlappedActor` OtherActor _asbp_pc_main_controller)
      (set `/Game/Blueprints/Framework/BP_PC_MainController.OverlappedComponent` OverlappedComponent _asbp_pc_main_controller)
      (`/Game/Blueprints/Framework/BP_PC_MainController.Server_AddFlowerUI` _asbp_pc_main_controller))))

(event `self.Collision_Sphere.OnComponentEndOverlap`
  (params (OverlappedComponent :type "PrimitiveComponent Object Reference") (OtherActor :type "Actor Object Reference") (OtherComp :type "PrimitiveComponent Object Reference") (OtherBodyIndex :type Integer))
  ;[1 1 1] End Overlap
  (`/Engine/EditorBlueprintResources/ActorMacros.Switch Has Authority`
    (:`Authority`
      (bind _asbp_pc_main_controller (cast `/Game/Blueprints/Framework/BP_PC_MainController` (`self.GetInstigatorController` OtherActor)))
      (bind _asbp_third_person_character (cast `/Game/Blueprints/Character/BP_ThirdPerson_Character` OtherActor))
      (set `/Game/Blueprints/Framework/BP_PC_MainController.DrySpot_OverlappedActor` null _asbp_pc_main_controller)
      (set `/Game/Blueprints/Framework/BP_PC_MainController.OverlappedComponent` null _asbp_pc_main_controller)
      (`/Game/Blueprints/Framework/BP_PC_MainController.Server_RemoveFlowerUI` _asbp_pc_main_controller)
      (`SceneComponent.SetVisibility` (`/Game/Blueprints/Character/BP_ThirdPerson_Character.FlowerSpawn` _asbp_third_person_character) false false))))

(fn `UserConstructionScript`)