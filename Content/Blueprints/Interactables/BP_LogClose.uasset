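; BP_LogClose is an interactable log Blueprint that configures an InterpToMovement component for a timed move along control points.
; The construction script loads the WayPoints variable as the path, sets the duration and turns off auto-activation.
; LogFall replaces that path with two relative points from Location1 and Location2 and resets the same duration.
; Neither graph starts the movement itself.
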(fn `LogFall`
  (bind _interptomovement (`self.InterpToMovement`))
  (set `InterpToMovementComponent.ControlPoints` (`|MakeArray` (make `InterpControlPoint` (`self.Location1`)) (make `InterpControlPoint` (`self.Location2`))) _interptomovement)
  (set `InterpToMovementComponent.Duration` 3.0 _interptomovement))

(fn `UserConstructionScript`
  (bind _interptomovement (`self.InterpToMovement`))
  (set `InterpToMovementComponent.ControlPoints` (`self.WayPoints`) _interptomovement)
  (set `InterpToMovementComponent.Duration` 3.0 _interptomovement)
  (`ActorComponent.SetAutoActivate` _interptomovement false))