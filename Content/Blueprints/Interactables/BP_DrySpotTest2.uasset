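; Test dry spot interactable that tracks, on the server, whether players are standing on it.
; The P2 spawn area's overlap events set OverlappingSpot on the overlapping character's BP_Default_PlayerState.
; Custom events set P1IsOnDrySpot by matching controllers against the game mode's Player1Indexes, but nothing here calls them and the P1 area's overlap events are empty.
; Disconnected leftovers hold per-player variants and a key-gated BP_Flowers spawn.
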(event `self.Collision_P2SpawnArea.OnComponentBeginOverlap`
  (params (OverlappedComponent :type "PrimitiveComponent Object Reference") (OtherActor :type "Actor Object Reference") (OtherComp :type "PrimitiveComponent Object Reference") (OtherBodyIndex :type Integer) (bFromSweep :type Boolean) (SweepResult :type "HitResult Structure (by ref)"))
  ;[1 1 1] Begin Overlap
  (`/Engine/EditorBlueprintResources/ActorMacros.Switch Has Authority`
    (:`Authority`
      (bind _asbp_third_person_character (cast `/Game/Blueprints/Character/BP_ThirdPerson_Character` OtherActor)) ; Get the Player State of the overlapping Character
      (bind _asbp_default_player_state (cast `/Game/Blueprints/Framework/BP_Default_PlayerState` (`Pawn.PlayerState` _asbp_third_person_character))) ; Set variables for that Player
      (`KismetSystemLibrary.PrintString` (`KismetSystemLibrary.GetDisplayName` _asbp_default_player_state))
      (set `/Game/Blueprints/Framework/BP_Default_PlayerState.OverlappingSpot?` true _asbp_default_player_state))))

(event `self.Collision_P2SpawnArea.OnComponentEndOverlap`
  (params (OverlappedComponent :type "PrimitiveComponent Object Reference") (OtherActor :type "Actor Object Reference") (OtherComp :type "PrimitiveComponent Object Reference") (OtherBodyIndex :type Integer))
  ;[1 1 1] End Overlap
  (`/Engine/EditorBlueprintResources/ActorMacros.Switch Has Authority`
    (:`Authority`
      (bind _asbp_third_person_character (cast `/Game/Blueprints/Character/BP_ThirdPerson_Character` OtherActor))
      (bind _asbp_default_player_state (cast `/Game/Blueprints/Framework/BP_Default_PlayerState` (`Pawn.PlayerState` _asbp_third_person_character)))
      (`KismetSystemLibrary.PrintString` (`KismetSystemLibrary.GetDisplayName` _asbp_default_player_state))
      (set `/Game/Blueprints/Framework/BP_Default_PlayerState.OverlappingSpot?` false _asbp_default_player_state))))

(event `CustomEvent`
  (params (OverlappedComponent :type "PrimitiveComponent Object Reference") (OtherActor :type "Actor Object Reference") (OtherComp :type "PrimitiveComponent Object Reference") (OtherBodyIndex :type Integer) (bFromSweep :type Boolean) (SweepResult :type "HitResult Structure (by ref)"))
  (bind _returnvalue (`self.GetInstigatorController` OtherActor))
  ;[1 0.4308 0.9567] Player 1 (Client)
  ;;[1 1 1] Begin Overlap
  (`/Engine/EditorBlueprintResources/ActorMacros.Switch Has Authority`
    (:`Authority`
      (bind _asbp_pc_main_controller (cast `/Game/Blueprints/Framework/BP_PC_MainController` _returnvalue))
      (set `self.P1_PC_DrySpot` _returnvalue)
      (bind _asbp_gm_default (cast `/Game/Blueprints/Framework/BP_GM_Default` (`GameplayStatics.GetGameMode`)))
      (for _array_element (`/Game/Blueprints/Framework/BP_GM_Default.Player1Indexes` _asbp_gm_default)
        (if (== (`KismetArrayLibrary.Array_Find` (`/Game/Blueprints/Framework/BP_GM_Default.AllPlayerControllers` _asbp_gm_default) _asbp_pc_main_controller) _array_element)
          (set `self.P1_IsOnDrySpot?` true)
          (`KismetSystemLibrary.PrintString` "Player 1 on dry spot"))))))

(event `self.Collision_P1SpawnArea.OnComponentBeginOverlap`
  (params (OverlappedComponent :type "PrimitiveComponent Object Reference") (OtherActor :type "Actor Object Reference") (OtherComp :type "PrimitiveComponent Object Reference") (OtherBodyIndex :type Integer) (bFromSweep :type Boolean) (SweepResult :type "HitResult Structure (by ref)"))
  ;[1 0.4308 0.9567] Player 1 (Client)
  ;;[1 1 1] Begin Overlap
)

(event `CustomEvent_1`
  (params (OverlappedComponent :type "PrimitiveComponent Object Reference") (OtherActor :type "Actor Object Reference") (OtherComp :type "PrimitiveComponent Object Reference") (OtherBodyIndex :type Integer))
  ;[1 0.4308 0.9567] Player 1 (Client)
  ;;[1 1 1] End Overlap
  (`/Engine/EditorBlueprintResources/ActorMacros.Switch Has Authority`
    (:`Authority`
      (bind _asbp_pc_main_controller (cast `/Game/Blueprints/Framework/BP_PC_MainController` (`self.GetInstigatorController` OtherActor)))
      (bind _asbp_gm_default (cast `/Game/Blueprints/Framework/BP_GM_Default` (`GameplayStatics.GetGameMode`)))
      (for _array_element (`/Game/Blueprints/Framework/BP_GM_Default.Player1Indexes` _asbp_gm_default)
        (if (== (`KismetArrayLibrary.Array_Find` (`/Game/Blueprints/Framework/BP_GM_Default.AllPlayerControllers` _asbp_gm_default) _asbp_pc_main_controller) _array_element)
          (set `self.P1_IsOnDrySpot?` false)
          (`KismetSystemLibrary.PrintString` "Player 1 is not on dry spot"))))))

(event `self.Collision_P1SpawnArea.OnComponentEndOverlap`
  (params (OverlappedComponent :type "PrimitiveComponent Object Reference") (OtherActor :type "Actor Object Reference") (OtherComp :type "PrimitiveComponent Object Reference") (OtherBodyIndex :type Integer))
  ;[1 0.4308 0.9567] Player 1 (Client)
  ;;[1 1 1] End Overlap
)

(fn `UserConstructionScript`)