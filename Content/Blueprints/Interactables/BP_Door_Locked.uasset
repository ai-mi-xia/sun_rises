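; BP_Door_Locked is a locked door interactable that handles a player UI message and opening, with logic gated to the server.
; Box overlaps call ClientShowMessageUI on BP_PC_MainController to toggle the message, though a constant-true branch prevents the show call.
; OpenDoor destroys the actor and then plays a 2D sound.
; The HasKey check is unfinished and disconnected, so no key is verified here.
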(event `self.Box_collision.OnComponentBeginOverlap`
  (params (OverlappedComponent :type "PrimitiveComponent Object Reference") (OtherActor :type "Actor Object Reference") (OtherComp :type "PrimitiveComponent Object Reference") (OtherBodyIndex :type Integer) (bFromSweep :type Boolean) (SweepResult :type "HitResult Structure (by ref)"))
  ;[1 1 1] Overlap Door Collision
  (`/Engine/EditorBlueprintResources/ActorMacros.Switch Has Authority`
    (:`Authority`
      ;;[1 0.5573 0.5573] Is the door open?
      (if (not (`self.doorOpen`))
        (bind _asbp_pc_main_controller (cast `/Game/Blueprints/Framework/BP_PC_MainController` (`self.GetInstigatorController` OtherActor)))
        (if (not true)
          (`/Game/Blueprints/Framework/BP_PC_MainController.Client_ShowMessageUI` _asbp_pc_main_controller true))))))

(event `self.Box_collision.OnComponentEndOverlap`
  (params (OverlappedComponent :type "PrimitiveComponent Object Reference") (OtherActor :type "Actor Object Reference") (OtherComp :type "PrimitiveComponent Object Reference") (OtherBodyIndex :type Integer))
  ;[1 1 1] End Overlap Door Collision - remove message
  (`/Engine/EditorBlueprintResources/ActorMacros.Switch Has Authority`
    (:`Authority`
      (bind _asbp_pc_main_controller (cast `/Game/Blueprints/Framework/BP_PC_MainController` (`self.GetInstigatorController` OtherActor)))
      (`/Game/Blueprints/Framework/BP_PC_MainController.Client_ShowMessageUI` _asbp_pc_main_controller false))))

(event `OpenDoor`
  ;[1 1 1] Open Door Event
  (`/Engine/EditorBlueprintResources/ActorMacros.Switch Has Authority`
    (:`Authority`
      (`self.K2_DestroyActor`)
      (`GameplayStatics.PlaySound2D` "/Game/Assets/Audio/SFX_door_locked.SFX_door_locked" 1.0 1.0 0.0 null null))))

(fn `UserConstructionScript`)