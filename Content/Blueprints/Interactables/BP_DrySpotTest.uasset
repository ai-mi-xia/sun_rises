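; Test interactable that tracks whether Player 1 and Player 2 are standing on their dry spots.
; Each player's collision area sets or clears that player's flag on overlap, with authority only.
; Players are identified by looking up the instigator controller's index in the game mode's per-player index lists.
; Debug prints, duplicate Player 1 custom events with no visible caller, and disconnected logic, including a flower spawn, remain in the graph.
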(event `self.Collision_P2SpawnArea.OnComponentBeginOverlap`
  (params (OverlappedComponent :type "PrimitiveComponent Object Reference") (OtherActor :type "Actor Object Reference") (OtherComp :type "PrimitiveComponent Object Reference") (OtherBodyIndex :type Integer) (bFromSweep :type Boolean) (SweepResult :type "HitResult Structure (by ref)"))
  (bind _returnvalue (`self.GetInstigatorController` OtherActor))
  ;[0.4651 0.9402 1] Player 2 (Server)
  ;;[1 1 1] Begin Overlap
  (`/Engine/EditorBlueprintResources/ActorMacros.Switch Has Authority`
    (:`Authority`
      (set `self.Overlapping Actor P2` OtherActor)
      (bind _asbp_pc_main_controller (cast `/Game/Blueprints/Framework/BP_PC_MainController` _returnvalue))
      (bind _output_get (set `self.P2_OverlappedPC` _returnvalue))
      (`KismetSystemLibrary.PrintString` (`KismetSystemLibrary.GetDisplayName` _output_get))
      (bind _asbp_gm_default (cast `/Game/Blueprints/Framework/BP_GM_Default` (`GameplayStatics.GetGameMode`)))
      (for _array_element (`/Game/Blueprints/Framework/BP_GM_Default.Player2Indexes` _asbp_gm_default)
        (if (== (`KismetArrayLibrary.Array_Find` (`/Game/Blueprints/Framework/BP_GM_Default.AllPlayerControllers` _asbp_gm_default) _asbp_pc_main_controller) _array_element)
          (set `self.P2_IsOnDrySpot?` true))))))

(event `self.Collision_P2SpawnArea.OnComponentEndOverlap`
  (params (OverlappedComponent :type "PrimitiveComponent Object Reference") (OtherActor :type "Actor Object Reference") (OtherComp :type "PrimitiveComponent Object Reference") (OtherBodyIndex :type Integer))
  ;[0.4651 0.9402 1] Player 2 (Server)
  ;;[1 1 1] End Overlap
  (`/Engine/EditorBlueprintResources/ActorMacros.Switch Has Authority`
    (:`Authority`
      (bind _asbp_pc_main_controller (cast `/Game/Blueprints/Framework/BP_PC_MainController` (`self.GetInstigatorController` OtherActor)))
      (bind _asbp_gm_default (cast `/Game/Blueprints/Framework/BP_GM_Default` (`GameplayStatics.GetGameMode`)))
      (for _array_element (`/Game/Blueprints/Framework/BP_GM_Default.Player2Indexes` _asbp_gm_default)
        (if (== (`KismetArrayLibrary.Array_Find` (`/Game/Blueprints/Framework/BP_GM_Default.AllPlayerControllers` _asbp_gm_default) _asbp_pc_main_controller) _array_element)
          (set `self.P2_IsOnDrySpot?` false)
          (`KismetSystemLibrary.PrintString` "Player 2 is not on dry spot"))))))

(event `CustomEvent`
  (params (OverlappedComponent :type "PrimitiveComponent Object Reference") (OtherActor :type "Actor Object Reference") (OtherComp :type "PrimitiveComponent Object Reference") (OtherBodyIndex :type Integer) (bFromSweep :type Boolean) (SweepResult :type "HitResult Structure (by ref)"))
  (bind _returnvalue (`self.GetInstigatorController` OtherActor))
  ;[1 0.4308 0.9567] Player 1 (Client)
  ;;[1 1 1] Begin Overlap
  (`/Engine/EditorBlueprintResources/ActorMacros.Switch Has Authority`
    (:`Authority`
      (bind _asbp_pc_main_controller (cast `/Game/Blueprints/Framework/BP_PC_MainController` _returnvalue))
      (set `self.P1_PC_DrySpot` _returnvalue)
      (bind _asbp_gm_default (cast `/Game/Blueprints/Framework/BP_GM_Default` (`GameplayStatics.GetGameMode`)))
      (for _array_element (`/Game/Blueprints/Framework/BP_GM_Default.Player1Indexes` _asbp_gm_default)
        (if (== (`KismetArrayLibrary.Array_Find` (`/Game/Blueprints/Framework/BP_GM_Default.AllPlayerControllers` _asbp_gm_default) _asbp_pc_main_controller) _array_element)
          (set `self.P1_IsOnDrySpot?` true)
          (`KismetSystemLibrary.PrintString` "Player 1 on dry spot"))))))

(event `self.Collision_P1SpawnArea.OnComponentBeginOverlap`
  (params (OverlappedComponent :type "PrimitiveComponent Object Reference") (OtherActor :type "Actor Object Reference") (OtherComp :type "PrimitiveComponent Object Reference") (OtherBodyIndex :type Integer) (bFromSweep :type Boolean) (SweepResult :type "HitResult Structure (by ref)"))
  (bind _returnvalue (`self.GetInstigatorController` OtherActor))
  ;[1 0.4308 0.9567] Player 1 (Client)
  ;;[1 1 1] Begin Overlap
  (`/Engine/EditorBlueprintResources/ActorMacros.Switch Has Authority`
    (:`Authority`
      (set `self.Overlapping Actor P1` OtherActor)
      (bind _asbp_pc_main_controller (cast `/Game/Blueprints/Framework/BP_PC_MainController` _returnvalue))
      (bind _output_get (set `self.P1_OverlappedPC` _returnvalue))
      (`KismetSystemLibrary.PrintString` (`KismetSystemLibrary.GetDisplayName` _output_get))
      (bind _asbp_gm_default (cast `/Game/Blueprints/Framework/BP_GM_Default` (`GameplayStatics.GetGameMode`)))
      (for _array_element (`/Game/Blueprints/Framework/BP_GM_Default.Player1Indexes` _asbp_gm_default)
        (if (== (`KismetArrayLibrary.Array_Find` (`/Game/Blueprints/Framework/BP_GM_Default.AllPlayerControllers` _asbp_gm_default) _asbp_pc_main_controller) _array_element)
          (set `self.P1_IsOnDrySpot?` true))))))

(event `CustomEvent_1`
  (params (OverlappedComponent :type "PrimitiveComponent Object Reference") (OtherActor :type "Actor Object Reference") (OtherComp :type "PrimitiveComponent Object Reference") (OtherBodyIndex :type Integer))
  ;[1 0.4308 0.9567] Player 1 (Client)
  ;;[1 1 1] End Overlap
  (`/Engine/EditorBlueprintResources/ActorMacros.Switch Has Authority`
    (:`Authority`
      (bind _asbp_pc_main_controller (cast `/Game/Blueprints/Framework/BP_PC_MainController` (`self.GetInstigatorController` OtherActor)))
      (bind _asbp_gm_default (cast `/Game/Blueprints/Framework/BP_GM_Default` (`GameplayStatics.GetGameMode`)))
      (for _array_element (`/Game/Blueprints/Framework/BP_GM_Default.Player1Indexes` _asbp_gm_default)
        (if (== (`KismetArrayLibrary.Array_Find` (`/Game/Blueprints/Framework/BP_GM_Default.AllPlayerControllers` _asbp_gm_default) _asbp_pc_main_controller) _array_element)
          (set `self.P1_IsOnDrySpot?` false)
          (`KismetSystemLibrary.PrintString` "Player 1 is not on dry spot"))))))

(event `self.Collision_P1SpawnArea.OnComponentEndOverlap`
  (params (OverlappedComponent :type "PrimitiveComponent Object Reference") (OtherActor :type "Actor Object Reference") (OtherComp :type "PrimitiveComponent Object Reference") (OtherBodyIndex :type Integer))
  ;[1 0.4308 0.9567] Player 1 (Client)
  ;;[1 1 1] End Overlap
  (`/Engine/EditorBlueprintResources/ActorMacros.Switch Has Authority`
    (:`Authority`
      (bind _asbp_pc_main_controller (cast `/Game/Blueprints/Framework/BP_PC_MainController` (`self.GetInstigatorController` OtherActor)))
      (bind _asbp_gm_default (cast `/Game/Blueprints/Framework/BP_GM_Default` (`GameplayStatics.GetGameMode`)))
      (for _array_element (`/Game/Blueprints/Framework/BP_GM_Default.Player1Indexes` _asbp_gm_default)
        (if (== (`KismetArrayLibrary.Array_Find` (`/Game/Blueprints/Framework/BP_GM_Default.AllPlayerControllers` _asbp_gm_default) _asbp_pc_main_controller) _array_element)
          (set `self.P1_IsOnDrySpot?` false))))))

(fn `UserConstructionScript`)