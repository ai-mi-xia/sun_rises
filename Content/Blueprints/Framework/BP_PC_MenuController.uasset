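; Player controller for menu and lobby maps that sets up UI-only mouse input for the local player and manages the lobby screen.
; It creates the lobby widget once, caches it and adds it to the viewport on request.
; Server and client events find that widget to change its waiting text, with the server event also calling the client one.
; Ending a client session destroys it and opens the main menu map.
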(event `self.ReceiveBeginPlay`
  ;[1 1 1] Setup
  (if (`self.IsLocalController`)
    (set `self.bShowMouseCursor` true)
    (`WidgetBlueprintLibrary.SetInputMode_UIOnlyEx` self null)))

(event `EndClientSession`
  ;[1 1 1] For Lobby Map
  (`DestroySessionCallbackProxy.DestroySession` self
    (:`OnSuccess`
      (`GameplayStatics.OpenLevel` "MainMenu_Map"))))

(event `Create_LobbyMenu`
  ;[1 1 1] Show Lobby UI on each client
  (`self.UIShowLobbyMenu`))

(event `Server_UIChangeWaitingText`
  ;[1 1 1] Change Waiting Text to Loading on Lobby WBP (currently not working if i only call on client
  (bind _foundwidgets (`WidgetBlueprintLibrary.GetAllWidgetsOfClass` "/Game/Widgets/Menu_and_Lobby/Lobby_WidgetBP.Lobby_WidgetBP_C"))
  (bind _aslobby_widget_bp (cast `/Game/Widgets/Menu_and_Lobby/Lobby_WidgetBP` (`|GetArrayItem` _foundwidgets)))
  (`/Game/Widgets/Menu_and_Lobby/Lobby_WidgetBP.ChangeWaitingText` _aslobby_widget_bp)
  (`self.Client_UIChangeWaitingText`))

(event `Client_UIChangeWaitingText`
  ;[1 1 1] Change Waiting Text to Loading on Lobby WBP (currently not working if i only call on client
  (bind _foundwidgets (`WidgetBlueprintLibrary.GetAllWidgetsOfClass` "/Game/Widgets/Menu_and_Lobby/Lobby_WidgetBP.Lobby_WidgetBP_C"))
  (bind _aslobby_widget_bp (cast `/Game/Widgets/Menu_and_Lobby/Lobby_WidgetBP` (`|GetArrayItem` _foundwidgets)))
  (`/Game/Widgets/Menu_and_Lobby/Lobby_WidgetBP.ChangeWaitingText` _aslobby_widget_bp))

(fn `UIShowLobbyMenu`
  (`/Engine/EditorBlueprintResources/StandardMacros.IsValid` (`self.WBP_Lobby`)
    (:`Is Valid`
      _)
    (:`Is Not Valid`
      (bind _returnvalue (`|CreateWidget` "/Game/Widgets/Menu_and_Lobby/Lobby_WidgetBP.Lobby_WidgetBP_C" self))
      (set `self.WBP_Lobby` _returnvalue)))
  (`UserWidget.AddToViewport` (`self.WBP_Lobby`) 0)
  (return))

(fn `UserConstructionScript`)