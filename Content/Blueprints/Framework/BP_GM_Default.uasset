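; Default game mode that tracks connected main player controllers and triggers player list refreshes as players join or leave.
; On login it stores the controller and tells the client to draw its HUD; on logout it removes it.
; The list update waits briefly, then delegates to the GameState.
; An unfinished Respawn event forwards to the controller's server respawn, and player start selection is left unused.
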(event `self.K2_PostLogin`
  (params (NewPlayer :type "PlayerController Object Reference"))
  ;[1 1 1] Every time player joins game, tell player controller to create HUD
  (bind _asbp_pc_main_controller (cast `/Game/Blueprints/Framework/BP_PC_MainController` NewPlayer))
  (`KismetArrayLibrary.Array_Add` (`self.AllPlayerControllers`) _asbp_pc_main_controller)
  (bind _outactors (`GameplayStatics.GetAllActorsOfClass` "/Game/Blueprints/Framework/PlayerStart_Blueprint.PlayerStart_Blueprint_C"))
  (`/Game/Blueprints/Framework/BP_PC_MainController.Client_DrawHUD` _asbp_pc_main_controller)
  (`self.Update_PlayerList` :!label _label))

(event `self.K2_OnLogout`
  (params (ExitingController :type "Controller Object Reference"))
  ;[1 1 1] Remove players from array on disconnect
  (bind _asbp_pc_main_controller (cast `/Game/Blueprints/Framework/BP_PC_MainController` ExitingController))
  (`KismetArrayLibrary.Array_RemoveItem` (`self.AllPlayerControllers`) _asbp_pc_main_controller)
  (goto _label))

(event `Update_PlayerList`
  ;[1 1 1] make gamestate responsible for updating player list (rep on client and server)
  (`KismetSystemLibrary.Delay` 0.3)
  (bind _asbp_game_state_base (cast `/Game/Blueprints/Framework/BP_GameStateBase` (`GameplayStatics.GetGameState`)))
  (`/Game/Blueprints/Framework/BP_GameStateBase.Update_PlayerList` _asbp_game_state_base))

(event `Respawn`
  (params (Controller :type "Controller Object Reference"))
  ;[1 0.5104 0.5104] unfinished  - respawn
  (bind _asbp_pc_main_controller (cast `/Game/Blueprints/Framework/BP_PC_MainController` Controller))
  (`/Game/Blueprints/Framework/BP_PC_MainController.Server_Respawn` :`self` _asbp_pc_main_controller))

(fn `UserConstructionScript`)